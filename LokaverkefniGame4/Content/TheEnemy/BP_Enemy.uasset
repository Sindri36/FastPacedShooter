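; Enemy actor that chases the first-person player and, when killed, notifies the level's door and is replaced by a BP_Enemy_2.
; PawnSensing sightings drive AI MoveTo, while damage drains Health until Death runs.
; Death calls TryToOpenDoor on the Door_Bp found at BeginPlay, spawns the successor at its transform, then destroys itself.
; A disconnected ragdoll and traced Niagara blood-pool sequence never runs.
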(event OnSeePawn(PawnSensing)
  (params (Pawn :type Pawn%20Object%20Reference))
  ;[1 1 1] Enemy move
  (bind _asbp_first_person_character (Utilities|Casting|CastToBP_FirstPersonCharacter Pawn))
  (AI|AIMoveTo self "0, 0, 0" _asbp_first_person_character 5.0 false))

(event Custom|Death
  (Default|TrytoOpenDoor (Variables|Default|GetDoorRef))
  (Game|SpawnActorfromClass "/Game/TheEnemy/BP_Enemy_2.BP_Enemy_2_C" (Transformation|GetActorTransform) "Undefined" 0 0)
  (Actor|DestroyActor))

(event EventBeginPlay
  (bind _returnvalue (Actor|GetActorOfClass "/Game/FirstPerson/Blueprints/Door_Bp.Door_Bp_C"))
  (Variables|Default|SetDoorRef _returnvalue))

(event Collision|EventActorBeginOverlap
  (params (OtherActor :type Actor%20Object%20Reference)))

(event EventTick
  (params (DeltaSeconds :type Float%20%28single-precision%29)))

(event Game|Damage|EventAnyDamage
  (params (Damage :type Float%20%28single-precision%29) (DamageType :type Damage%20Type%20Object%20Reference) (InstigatedBy :type Controller%20Object%20Reference) (DamageCauser :type Actor%20Object%20Reference))
  ;[1 1 1] EnemyGetShot and collision particle stuff
  (if (> (Variables|Default|GetHealth) 0.0)
    (bind _output_get (Variables|Default|SetHealth (- (Variables|Default|GetHealth) Damage)))
    (if (<= _output_get 0.0)
      (CallFunction|Death))))

(fn ConstructionScript)