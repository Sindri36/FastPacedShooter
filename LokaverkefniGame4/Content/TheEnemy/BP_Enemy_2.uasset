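; BP_Enemy_2 is an enemy that collapses into a ragdoll as soon as play begins and leaves a blood pool.
; BeginPlay enables physics on the mesh and disables capsule collision.
; After a short delay, it line-traces vertically through the spine bone to find a surface, with persistent debug drawing.
; It spawns the Niagara blood pool at the hit point, aligned to the impact normal, without checking for a hit.
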(event EventBeginPlay
  (bind _mesh (Variables|Character|GetMesh))
  (bind _returnvalue (Transformation|GetSocketLocation _mesh "spine_02"))
  ;[1 1 1] EnemyGetShot and collision particle stuff
  (Physics|SetSimulatePhysics _mesh true)
  (Collision|SetCollisionEnabled (Variables|Collision|GetCapsuleComponent) "NoCollision")
  (Utilities|FlowControl|Delay 1.5)
  (bind _outhit (Collision|LineTraceByChannel (+ _returnvalue "0.000000,0.000000,250.000000") (+ _returnvalue "0.000000,0.000000,-250.000000") "TraceTypeQuery1" false (Variables|Default|GetActorTolgnore) "Persistent"))
  (Niagara|SpawnSystematLocation "/Game/BloodPartivle/BloodPoolNiagara.BloodPoolNiagara" (.Location (Collision|BreakHitResult _outhit)) (Math|Conversions|RotationFromXVector (.ImpactNormal (Collision|BreakHitResult _outhit)))))

(event Collision|EventActorBeginOverlap
  (params (OtherActor :type Actor%20Object%20Reference)))

(event EventTick
  (params (DeltaSeconds :type Float%20%28single-precision%29)))

(fn ConstructionScript)